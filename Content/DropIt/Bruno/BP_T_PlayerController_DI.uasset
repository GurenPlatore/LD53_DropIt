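; Player controller for DropIt that drives a free-roaming camera through the BP_T_PlayerPOV pawn and its spring arm, cached on BeginPlay.
; Movement axes and screen-edge mouse scrolling on Tick feed MoveCamera, which offsets the pawn relative to its rotation, without sweeping.
; A rotation axis or right-mouse drag yaws the pawn, while right-mouse drag also tilts the spring arm within a clamped pitch.
; Zoom actions step the clamped arm length.
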(event `InputAxis|RotateCamUpDown`
  (params (AxisValue :type "Float (single-precision)"))
  (bind _spring_arm (`self.Spring Arm`))
  (bind (_relativerotation_roll _relativerotation_pitch) (`KismetMathLibrary.BreakRotator` (`SceneComponent.RelativeRotation` _spring_arm)))
  (if (`self.IsInputKeyDown` "RightMouseButton")
    (`SceneComponent.K2_AddLocalRotation` _spring_arm (`KismetMathLibrary.MakeRotator` 0.0 (- (`KismetMathLibrary.FClamp` (+ _relativerotation_pitch (* AxisValue 500.0 (`GameplayStatics.GetWorldDeltaSeconds`))) -90.0) _relativerotation_pitch)) false false)))

(event `InputAxis|RotateCamLeftRight`
  (params (AxisValue :type "Float (single-precision)"))
  (if (`self.IsInputKeyDown` "RightMouseButton")
    (`self.K2_AddActorWorldRotation` (`self.K2_GetPawn`) (`KismetMathLibrary.MakeRotator` 0.0 0.0 (* AxisValue 500.0 (`GameplayStatics.GetWorldDeltaSeconds`))) false false)))

(event `InputAxis|RotateCameraInput`
  (params (AxisValue :type "Float (single-precision)"))
  ;[1 1 1] RotateCamera
  (`self.K2_AddActorWorldRotation` (`self.K2_GetPawn`) (`KismetMathLibrary.MakeRotator` 0.0 0.0 (* AxisValue (`self.CameraRotationSpeed`) (`GameplayStatics.GetWorldDeltaSeconds`))) false false))

(event `InputAction|ZoomIn`
  (params (Key :type "Key Structure"))
  (bind _spring_arm (`self.Spring Arm`))
  ;[1 1 1] Zoom
  (:`Pressed`
    (set `SpringArmComponent.TargetArmLength` (`KismetMathLibrary.FClamp` (- (`SpringArmComponent.TargetArmLength` _spring_arm) (`self.ZoomSpeed`)) 0.0 1200.0) _spring_arm)))

(event `InputAxis|MoveForward`
  (params (AxisValue :type "Float (single-precision)"))
  ;[1 1 1] ZQSD Movevement
  (`self.MoveCamera` (`KismetMathLibrary.MakeVector` (* AxisValue (* (`GameplayStatics.GetWorldDeltaSeconds`) (`self.CameraScrollSpeed`)) 1.0))))

(event `self.ReceiveBeginPlay`
  (bind _asbp_t_player_pov (cast `/Game/DropIt/Bruno/BP_T_PlayerPOV` (`self.K2_GetPawn`)))
  (set `self.Spring Arm` (`/Game/DropIt/Bruno/BP_T_PlayerPOV.SpringArm` _asbp_t_player_pov)))

(event `InputAction|ZoomOut`
  (params (Key :type "Key Structure"))
  (bind _spring_arm (`self.Spring Arm`))
  ;[1 1 1] Zoom
  (:`Pressed`
    (set `SpringArmComponent.TargetArmLength` (`KismetMathLibrary.FClamp` (+ (`SpringArmComponent.TargetArmLength` _spring_arm) (`self.ZoomSpeed`)) 0.0 1200.0) _spring_arm)))

(event `InputAxis|MoveRight`
  (params (AxisValue :type "Float (single-precision)"))
  ;[1 1 1] ZQSD Movevement
  (`self.MoveCamera` (`KismetMathLibrary.MakeVector` 0.0 (* AxisValue (* (`GameplayStatics.GetWorldDeltaSeconds`) (`self.CameraScrollSpeed`)) -1.0))))

(event `self.ReceiveTick`
  (params (DeltaSeconds :type "Float (single-precision)"))
  (bind _cameraedgescrollthreshold (`self.CameraEdgeScrollThreshold`))
  (bind _cameraedgescrollthreshold_2 (`self.CameraEdgeScrollThreshold`))
  ;[1 1 1] ScreenTouchMovement
  (set `self.CameraScrollSpeedFPS` (* DeltaSeconds (`self.CameraScrollSpeed`)))
  (bind _returnvalue (`WidgetLayoutLibrary.GetMousePositionOnViewport`))
  (bind _returnvalue_2 (`WidgetLayoutLibrary.GetViewportWidgetGeometry`))
  (`|ExecutionSequence`
    (:`then_0`
      (bind (_x _y) (`KismetMathLibrary.BreakVector2D` _returnvalue))
      (if (< _x _cameraedgescrollthreshold)
        (`self.MoveCamera` (`KismetMathLibrary.MakeVector` 0.0 (* (`self.CameraScrollSpeedFPS`) -1.0)))
        (else
          (bind (_x_2 _y_2) (`KismetMathLibrary.BreakVector2D` (`SlateBlueprintLibrary.GetLocalSize` _returnvalue_2)))
          (if (> _x (- _x_2 _cameraedgescrollthreshold))
            (`self.MoveCamera` (`KismetMathLibrary.MakeVector` 0.0 (`self.CameraScrollSpeedFPS`)))))))
    (:`then_1`
      (if (< _y _cameraedgescrollthreshold_2)
        (`self.MoveCamera` (`KismetMathLibrary.MakeVector` (`self.CameraScrollSpeedFPS`)))
        (elif (> _y (- _y_2 _cameraedgescrollthreshold_2))
          (`self.MoveCamera` (`KismetMathLibrary.MakeVector` (* (`self.CameraScrollSpeedFPS`) -1.0))))))))

(fn `MoveCamera`
  (params (B :type "Vector Structure"))
  (bind _returnvalue (`self.K2_GetPawn`))
  (`self.K2_SetActorLocation` _returnvalue (+ (`self.K2_GetActorLocation` _returnvalue) (`KismetMathLibrary.GreaterGreater_VectorRotator` B (`self.K2_GetActorRotation` _returnvalue))) false false))

(fn `UserConstructionScript`)