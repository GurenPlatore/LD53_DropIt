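; Player POV Blueprint for DropIt that lets the player inspect AI pawns and spawn drops at its own location.
; Left click traces under the cursor, stores the hit pawn's name from the Spawner's map plus its level, and briefly shows a hand cursor.
; Drop spawns at a fixed height, then a looping Delay runs the cooldown; early presses trigger an error sound and widget.
; BeginPlay creates the minimap and HUD, and also flashes the error widget.
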(event `Key|LeftMouseButton`
  (params (Key :type "Key Structure"))
  (bind _asbp_player_controller_di (cast `/Game/DropIt/Vasguen/Controller/BP_PlayerController_DI` (`GameplayStatics.GetPlayerController` 0) :!pure true))
  (bind (_hitresult _returnvalue) (`PlayerController.GetHitResultUnderCursorForObjects` (cast `/Game/DropIt/Vasguen/Controller/BP_PlayerController_DI` (`self.GetController`) :!pure true) (`|MakeArray` "ObjectTypeQuery3" :!type "EObjectTypeQuery Enum") true))
  ;[1 1 1] Click sur les objet
  (:`Pressed`
    (if _returnvalue
      (bind _asbp_iapawn (cast `/Game/DropIt/Patrick/Blueprints/BP_IAPawn` (`.HitActor` (`GameplayStatics.BreakHitResult` _hitresult))))
      (set `self.PlayerName` (`BlueprintMapLibrary.Map_Find` (`/Game/DropIt/Patrick/Blueprints/BP_Spawner.PawnMap` (`self.Spawner`)) _asbp_iapawn))
      (set `self.PlayerLevel` (`KismetStringLibrary.Concat_StrStr` "Level " ": " (`KismetStringLibrary.Conv_IntToString` (`/Game/DropIt/Patrick/Blueprints/BP_IAPawn.PawnLevel` _asbp_iapawn))))
      (set `PlayerController.CurrentMouseCursor` "Hand" _asbp_player_controller_di)
      (`KismetSystemLibrary.Delay` 0.2)
      (set `PlayerController.CurrentMouseCursor` "Default" _asbp_player_controller_di))))

(event `InputAction|Drop`
  (params (Key :type "Key Structure"))
  (bind (_returnvalue_x _returnvalue_y _returnvalue_z) (`KismetMathLibrary.BreakVector` (`self.K2_GetActorLocation`)))
  ;[1 1 1] Spaw drop et cooldown
  (:`Pressed`
    (if (`self.CanDrop?`)
      (bind _returnvalue (`|SpawnActorFromClass` "/Game/DropIt/Patrick/Blueprints/BP_Drop.BP_Drop_C" (`KismetMathLibrary.MakeTransform` (`KismetMathLibrary.MakeVector` _returnvalue_x _returnvalue_y _returnvalue_z)) "Undefined" "OverrideRootScale" null null))
      (`self.K2_SetActorLocation` _returnvalue (`KismetMathLibrary.MakeVector` _returnvalue_x _returnvalue_y 220.0) false false)
      (set `self.CanDrop?` false)
      (`KismetSystemLibrary.Delay` 1.0 :!label _label)
      (if (== (`self.TimeLeft`) 0.0)
        (set `self.CanDrop?` true)
        (set `self.TimeLeft` 10.0)
        (else
          (set `self.TimeLeft` (- (`self.TimeLeft`) 1.0))
          (goto _label)))
      (else
        ;;[1 1 1] ERROR
        (`GameplayStatics.PlaySound2D` "/Game/DropIt/Sound/S_Eerror.S_Eerror" 1.0 1.0 0.0 null null)
        (`UserWidget.AddToViewport` (stale `self.ReceiveBeginPlay` _returnvalue) 0 :!label _label_2)
        (`KismetSystemLibrary.Delay` 0.5)
        (`Widget.RemoveFromParent` (stale `self.ReceiveBeginPlay` _returnvalue))))))

(event `self.ReceiveBeginPlay`
  ;[1 1 1] Spaw drop et cooldown
  (`|ExecutionSequence`
    (:`then_0`
      ;;[1 1 1] ERROR
      (bind _returnvalue (`|CreateWidget` "/Game/DropIt/Vasguen/UI/U_error.U_error_C"))
      (goto _label_2))
    (:`then_1`
      ;;[1 1 1] Minimap
      (bind _returnvalue_2 (`|CreateWidget` "/Game/DropIt/Vasguen/Minimap/UI_Minimap.UI_Minimap_C"))
      (`UserWidget.AddToViewport` _returnvalue_2 0))
    (:`then_2`
      (bind _returnvalue_3 (`|CreateWidget` "/Game/DropIt/Vasguen/UI/U_HUD.U_HUD_C"))
      (`UserWidget.AddToViewport` _returnvalue_3 0))))

(fn `UserConstructionScript`)