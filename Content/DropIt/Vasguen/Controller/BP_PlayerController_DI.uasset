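; Player controller for a free camera that moves, rotates and zooms the possessed BP_PlayerPOV pawn, with the mouse cursor shown.
; Axis input pans through MoveCamera, which offsets the pawn relative to its rotation.
; Zoom changes the clamped spring arm length, keys yaw the pawn, and right-mouse drag yaws it or pitches the arm within limits.
; Screen-edge scrolling logic is present but disconnected, and Tick is empty.
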(event `self.ReceiveBeginPlay`
  (set `self.bShowMouseCursor` true)
  (bind _asbp_player_pov (cast `/Game/DropIt/Vasguen/Controller/BP_PlayerPOV` (`self.K2_GetPawn`)))
  (set `self.Spring Arm` (`/Game/DropIt/Vasguen/Controller/BP_PlayerPOV.SpringArm` _asbp_player_pov)))

(event `InputAction|ZoomIn`
  (params (Key :type "Key Structure"))
  (bind _spring_arm (`self.Spring Arm`))
  ;[1 1 1] Zoom
  (:`Pressed`
    (set `SpringArmComponent.TargetArmLength` (`KismetMathLibrary.FClamp` (- (`SpringArmComponent.TargetArmLength` _spring_arm) (`self.ZoomSpeed`)) -3000.0 2000.0) _spring_arm)))

(event `InputAxis|MoveForward`
  (params (AxisValue :type "Float (single-precision)"))
  ;[1 1 1] ZQSD Movevement
  (`self.MoveCamera` (`KismetMathLibrary.MakeVector` (* AxisValue (* (`GameplayStatics.GetWorldDeltaSeconds`) (`self.CameraScrollSpeed`)) 1.0))))

(event `InputAction|ZoomOut`
  (params (Key :type "Key Structure"))
  (bind _spring_arm (`self.Spring Arm`))
  ;[1 1 1] Zoom
  (:`Pressed`
    (set `SpringArmComponent.TargetArmLength` (`KismetMathLibrary.FClamp` (+ (`SpringArmComponent.TargetArmLength` _spring_arm) (`self.ZoomSpeed`)) -3000.0 2000.0) _spring_arm)))

(event `InputAxis|MoveRight`
  (params (AxisValue :type "Float (single-precision)"))
  ;[1 1 1] ZQSD Movevement
  (`self.MoveCamera` (`KismetMathLibrary.MakeVector` 0.0 (* AxisValue (* (`GameplayStatics.GetWorldDeltaSeconds`) (`self.CameraScrollSpeed`)) -1.0))))

(event `self.ReceiveTick`
  (params (DeltaSeconds :type "Float (single-precision)")))

(event `InputAxis|RotateCameraInput`
  (params (AxisValue :type "Float (single-precision)"))
  (bind _returnvalue (`self.K2_GetPawn`))
  (bind _returnvalue_2 (`self.K2_GetActorRotation` _returnvalue))
  ;[1 1 1] Rotation
  ;;[1 1 1] RotateCamera A/E Input
  (`self.K2_SetActorRotation` _returnvalue (`KismetMathLibrary.RLerp` _returnvalue_2 (`KismetMathLibrary.MakeRotator` 0.0 0.0 (+ (* AxisValue (`self.CameraRotationSpeed`) (`GameplayStatics.GetWorldDeltaSeconds`)) (.yaw _returnvalue_2))) 0.5 true) false))

(event `InputAxis|RotateCamUpDown`
  (params (AxisValue :type "Float (single-precision)"))
  (bind _spring_arm (`self.Spring Arm`))
  (bind (_relativerotation_roll _relativerotation_pitch) (`KismetMathLibrary.BreakRotator` (`SceneComponent.RelativeRotation` _spring_arm)))
  ;[1 1 1] Rotation
  ;;[1 1 1] Pitch/Yaw Rotation
  (if (`self.IsInputKeyDown` "RightMouseButton")
    (`SceneComponent.K2_AddLocalRotation` _spring_arm (`KismetMathLibrary.MakeRotator` 0.0 (- (`KismetMathLibrary.FClamp` (+ _relativerotation_pitch (* AxisValue (`self.CameraRotationSpeed`) (`GameplayStatics.GetWorldDeltaSeconds`))) -90.0) _relativerotation_pitch)) false false)))

(event `InputAxis|RotateCamLeftRight`
  (params (AxisValue :type "Float (single-precision)"))
  ;[1 1 1] Rotation
  ;;[1 1 1] Pitch/Yaw Rotation
  (if (`self.IsInputKeyDown` "RightMouseButton")
    (`self.K2_AddActorWorldRotation` (`self.K2_GetPawn`) (`KismetMathLibrary.MakeRotator` 0.0 0.0 (* AxisValue (`self.CameraRotationSpeed`) (`GameplayStatics.GetWorldDeltaSeconds`))) false false)))

(fn `MoveCamera`
  (params (B :type "Vector Structure"))
  (bind _returnvalue (`self.K2_GetPawn`))
  (`self.K2_SetActorLocation` _returnvalue (+ (`self.K2_GetActorLocation` _returnvalue) (`KismetMathLibrary.GreaterGreater_VectorRotator` B (`self.K2_GetActorRotation` _returnvalue))) false false))

(fn `UserConstructionScript`)