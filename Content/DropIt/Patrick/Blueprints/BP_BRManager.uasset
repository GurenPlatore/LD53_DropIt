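; BP_BRManager is an actor that continuously resizes a static mesh over time.
; Each tick it accumulates elapsed time and builds a target scale from it, with X fixed and Y and Z equal to the running total.
; The mesh's world scale eases toward that target through a fixed-alpha, frame-rate-dependent lerp.
; It also prints the elapsed time and current scale every frame.
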(event `self.ReceiveTick`
  (params (DeltaSeconds :type "Float (single-precision)"))
  (bind _staticmesh (`self.StaticMesh`))
  (bind _returnvalue (`SceneComponent.K2_GetComponentScale` _staticmesh))
  (bind _output_get (set `self.NewVar_0` (+ DeltaSeconds (`self.NewVar_0`))))
  (set `self.NewVar_1` (`KismetMathLibrary.MakeVector` 100.0 _output_get _output_get))
  (`KismetSystemLibrary.PrintString` (`KismetStringLibrary.Conv_DoubleToString` _output_get) true true (struct :`G` 1.0 :`B` 0.086323 :`A` 1.0) 2.0 "float")
  (`KismetSystemLibrary.PrintString` (`KismetStringLibrary.Conv_VectorToString` _returnvalue) true true (struct :`R` 1.0 :`G` 0.594639 :`A` 1.0) 2.0 "vector")
  (`SceneComponent.SetWorldScale3D` _staticmesh (`KismetMathLibrary.VLerp` _returnvalue (`self.NewVar_1`) 0.1)))

(fn `UserConstructionScript`)