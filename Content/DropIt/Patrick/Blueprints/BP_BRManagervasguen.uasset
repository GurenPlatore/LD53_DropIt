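; BP_BRManagervasguen is an actor, apparently a battle royale zone manager, that shrinks a static mesh in stages.
; Every ten seconds it sets a new target scale by subtracting ScaleModifier from the current scale and resets the blend alpha.
; Tick lerps from the mesh's current scale toward that target with the growing alpha, easing each step.
; Any BP_IAPawn that begins overlapping the mesh is killed through DieInFight.
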(event `self.ReceiveBeginPlay`
  (set `self.NewScale` (- (`SceneComponent.RelativeScale3D` (`self.StaticMesh`)) (`self.ScaleModifier`)) :!label _label)
  (`self.SetNewScale`))

(event `SetNewScale`
  (set `self.NewVar_0` 0.0)
  (`KismetSystemLibrary.Delay` 10.0)
  (goto _label))

(event `self.ReceiveTick`
  (params (DeltaSeconds :type "Float (single-precision)"))
  (bind _output_get (set `self.NewVar_0` (+ (/ DeltaSeconds 10.0) (`self.NewVar_0`))))
  (`SceneComponent.SetRelativeScale3D` (`self.StaticMesh`) (`KismetMathLibrary.VLerp` (`SceneComponent.RelativeScale3D` (`self.StaticMesh`)) (`self.NewScale`) (`KismetMathLibrary.FClamp` _output_get))))

(event `self.StaticMesh.OnComponentBeginOverlap`
  (params (OverlappedComponent :type "PrimitiveComponent Object Reference") (OtherActor :type "Actor Object Reference") (OtherComp :type "PrimitiveComponent Object Reference") (OtherBodyIndex :type Integer) (bFromSweep :type Boolean) (SweepResult :type "HitResult Structure (by ref)"))
  (bind _asbp_iapawn (cast `/Game/DropIt/Patrick/Blueprints/BP_IAPawn` OtherActor))
  (`/Game/DropIt/Patrick/Blueprints/BP_IAPawn.DieInFight` _asbp_iapawn))

(fn `UserConstructionScript`)