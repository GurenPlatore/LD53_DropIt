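; BP_IAPawn is an AI pawn that gets a random character mesh from a lookup map on BeginPlay and exposes perception state.
; Its DetectionBox overlaps record nearby BP_Drop and enemy BP_IAPawn references with in-range flags, although any other non-self actor also raises the enemy flag.
; Tick compares the current location with the previous frame's to set PawnIsMoving.
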(event `self.ReceiveBeginPlay`
  (set `self.NewVar_0` (`KismetMathLibrary.RandomIntegerInRange` 0 7))
  (`SkeletalMeshComponent.SetSkeletalMeshAsset` (`self.Mesh`) (`BlueprintMapLibrary.Map_Find` (`self.NewVar`) (`self.NewVar_0`))))

(event `self.DetectionBox.OnComponentBeginOverlap`
  (params (OverlappedComponent :type "PrimitiveComponent Object Reference") (OtherActor :type "Actor Object Reference") (OtherComp :type "PrimitiveComponent Object Reference") (OtherBodyIndex :type Integer) (bFromSweep :type Boolean) (SweepResult :type "HitResult Structure (by ref)"))
  (bind _asbp_drop (cast `/Game/DropIt/Patrick/Blueprints/BP_Drop` OtherActor)
    (:`then`
      (set `self.DropInRange` _asbp_drop)
      (set `self.DropIsInRange` true))
    (:`CastFailed`
      (if (!= self OtherActor)
        (set `self.EnnemyIsInRange` true)
        (bind _asbp_iapawn (cast `/Game/DropIt/Patrick/Blueprints/BP_IAPawn` OtherActor))
        (set `self.EnnemyAtRange` _asbp_iapawn)))))

(event `self.DetectionBox.OnComponentEndOverlap`
  (params (OverlappedComponent :type "PrimitiveComponent Object Reference") (OtherActor :type "Actor Object Reference") (OtherComp :type "PrimitiveComponent Object Reference") (OtherBodyIndex :type Integer))
  (cast `/Game/DropIt/Patrick/Blueprints/BP_IAPawn` OtherActor
    (:`then`
      (set `self.EnnemyIsInRange` false))
    (:`CastFailed`
      (cast `/Game/DropIt/Patrick/Blueprints/BP_Drop` OtherActor)
      (set `self.DropIsInRange` false))))

(event `self.ReceiveTick`
  (params (DeltaSeconds :type "Float (single-precision)"))
  (bind _output_get (set `self.PawnLocation` (`self.K2_GetActorLocation`)))
  (set `self.PawnIsMoving` (!= _output_get (`self.NewPawnLocation`)))
  (set `self.NewPawnLocation` (`self.PawnLocation`)))

(fn `UserConstructionScript`)