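; BP_Spawner populates the level with BP_IAPawn pawns, one at each entry in SpawnPoints.
; From BeginPlay it picks a random point, spawns a pawn at its location and removes that point from the array.
; Each pawn is stored in PawnMap under a label built from PlayerName and an incrementing PlayerNumber.
; After a short delay, the Spawner event loops back until no points remain.
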(event `self.ReceiveBeginPlay`
  (bind _output_get (set `self.ActorSpawned` (`|GetArrayItem` (`self.SpawnPoints`) (`KismetMathLibrary.RandomIntegerInRange` 0 (`KismetArrayLibrary.Array_LastIndex` (`self.SpawnPoints`)))) :!label _label))
  (bind _output_get_2 (set `self.NewVar_3` (`self.K2_GetActorLocation` _output_get)))
  (bind _returnvalue (`|SpawnActorFromClass` "/Game/DropIt/Patrick/Blueprints/BP_IAPawn.BP_IAPawn_C" (`KismetMathLibrary.MakeTransform` _output_get_2) "Undefined" "OverrideRootScale" null null))
  (bind _result (`/Engine/EditorBlueprintResources/StandardMacros.IncrementInt` (`self.PlayerNumber`))
    (:`  `
      (`BlueprintMapLibrary.Map_Add` (`self.PawnMap`) _returnvalue (`KismetStringLibrary.Concat_StrStr` (`self.PlayerName`) " : " (`KismetStringLibrary.Conv_IntToString` _result)))
      (`KismetArrayLibrary.Array_Remove` (`self.SpawnPoints`) (`KismetArrayLibrary.Array_Find` (`self.SpawnPoints`) (`self.ActorSpawned`)))
      (`KismetSystemLibrary.Delay` 0.2)
      (`self.Spawner`))))

(event `Spawner`
  (if (`KismetArrayLibrary.Array_IsNotEmpty` (`self.SpawnPoints`))
    (goto _label)))

(fn `UserConstructionScript`)